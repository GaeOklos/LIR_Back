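; BP_Light is an interactive-folder light actor whose spot light flickers at random while the game runs.
; On BeginPlay it stores the spot's intensity, then chains non-looping timers between on and off events.
; The light stays on for a random longer interval, drops to zero intensity for a very brief random blink, then restores the stored value and repeats indefinitely.
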(event Custom|ONLight
  (Rendering|Components|Light|SetIntensity (Variables|Default|GetSpot) (Variables|Default|GetIntensity))
  (CallFunction|StartWaitON))

(event Custom|StartWaitOFF
  (Utilities|Time|SetTimerbyEvent (delegate Custom|ONLight) (Math|Random|RandomFloatinRange 0.01 0.1)))

(event Custom|OFFLight
  (Rendering|Components|Light|SetIntensity (Variables|Default|GetSpot) 0.0)
  (CallFunction|StartWaitOFF))

(event Custom|Start%20WaitON
  (Utilities|Time|SetTimerbyEvent (delegate Custom|OFFLight) (Math|Random|RandomFloatinRange 0.5 3.0)))

(event EventBeginPlay
  (Variables|Default|SetIntensity (Variables|/Script/Engine.LightComponentBase|GetIntensity (Variables|Default|GetSpot)))
  (CallFunction|StartWaitON))

(fn ConstructionScript)