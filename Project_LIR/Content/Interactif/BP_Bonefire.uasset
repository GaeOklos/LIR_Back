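; BP_Bonefire is an interactable bonfire that serves as a rest and respawn checkpoint.
; On BeginPlay it caches the game mode and game instance; if flagged as main respawn point, it registers its RespawnPoint transform as the initial spawn one tick later.
; Interaction calls RestAtBonfire on the instigator, then after a short delay sets the respawn point and calls ReactivateBonefire on the game mode.
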(event EventStartInteraction
  (params (Instigator :type BP%20Player%20Object%20Reference))
  (Default|RestatBonfire Instigator)
  (Utilities|FlowControl|Delay 0.3)
  (Default|SetRespawnPoint (Variables|Default|GetAs%20GI%20Game%20Instance) (Transformation|GetWorldTransform (Variables|Default|GetRespawnPoint)))
  (Default|ReactivateBonefire (Variables|Default|GetAs%20GM%20Gameplay)))

(event EventBeginPlay
  (bind _asgm_gameplay (Utilities|Casting|CastToGM_gameplay (Game|GetGameMode)))
  (Variables|Default|SetAs%20GM%20Gameplay _asgm_gameplay)
  (bind _asgi_game_instance (Utilities|Casting|CastToGI_GameInstance (Game|GetGameInstance)))
  (Variables|Default|SetAs%20GI%20Game%20Instance _asgi_game_instance)
  (if (Variables|Default|GetMainRespawnPoint)
    (Utilities|FlowControl|DelayUntilNextTick)
    (Default|InitRespownPoint (Variables|Default|GetAs%20GI%20Game%20Instance) (Transformation|GetWorldTransform (Variables|Default|GetRespawnPoint)))))

(fn ConstructionScript)