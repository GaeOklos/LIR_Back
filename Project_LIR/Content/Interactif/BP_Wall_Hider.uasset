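; BP_Wall_Hider is an actor that hides a list of actors at night and shows them again during the day.
; An external caller fires START__HideActor with a NightTime flag, which loops over ActorToHide and sets each actor's hidden-in-game state.
; A stored Night boolean ensures the loop runs only when the day/night state actually changes.
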(event Custom|START__HideActor
  (params (night_Time? :type Boolean))
  (if night_Time?
    (if (not (Variables|Default|Getnight?))
      (Variables|Default|Setnight? true)
      (for _array_element (Variables|Default|GetActor_ToHide)
        (Rendering|SetActorHiddenInGame _array_element true)))
    (elif (Variables|Default|Getnight?)
      (Variables|Default|Setnight? false)
      (for _array_element_2 (Variables|Default|GetActor_ToHide)
        (Rendering|SetActorHiddenInGame _array_element_2 false)))))

(event EventBeginPlay)

(event Collision|EventActorBeginOverlap
  (params (OtherActor :type Actor%20Object%20Reference)))

(event EventTick
  (params (DeltaSeconds :type Float%20%28single-precision%29)))

(fn ConstructionScript)