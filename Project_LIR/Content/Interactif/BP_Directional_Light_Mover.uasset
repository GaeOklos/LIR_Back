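; BP_Directional_Light_Mover rotates an assigned directional light between its starting rotation and a final rotation to switch between day and night.
; BeginPlay caches the origin rotation, and a custom event receives the night flag, ignoring requests that match the current state.
; A timeline, with play rate set to the inverse of Speed, lerps the rotation along the shortest path, playing for night and reversing for day.
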(event Custom|START__Rotate_Sun
  (params (night_Time? :type Boolean))
  (Components|Timeline|SetPlayRate (Variables|Default|GetTIMER_Move_Sun) (/ 1.0 (Variables|Default|Getspeed)))
  (if night_Time?
    (if (not (Variables|Default|Getnight?))
      (Variables|Default|Setnight? true)
      (bind _alpha (Timeline|TIMER_Move_Sun Play)
        (:Update
          (Transformation|SetActorRotation (Variables|Default|GetDirection_Light_To_Move) (Math|Rotator|Lerp(Rotator) (Variables|Default|GetOrigin_Rotation) (Variables|Default|GetFina_Rotation) _alpha true)))))
    (elif (Variables|Default|Getnight?)
      (Variables|Default|Setnight? false)
      (Timeline|TIMER_Move_Sun Reverse))))

(event EventBeginPlay
  (Variables|Default|SetOrigin_Rotation (Transformation|GetActorRotation (Variables|Default|GetDirection_Light_To_Move))))

(fn ConstructionScript)