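; Player sword actor that deals light or heavy melee damage during an attack window opened by StartAttack and closed by StopAttack.
; While attacking, Tick sweeps a debug-drawn capsule trace forward from an Arrow component.
; Hit actors implementing BPI_Damageable receive PlayerStats base damage times the attack's multiplier, flagged as player physical damage.
; An ignore list, cleared at each attack start, limits each target to one hit per swing.
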(event Custom|StopAttack
  (Variables|Default|SetIsAttacking false))

(event Custom|StartAttack
  (params (AttackNumber :type Integer) (PlayerRef :type Actor%20Object%20Reference) (DamageMultiplicator :type Float%20%28double-precision%29) (IsHeavy :type Boolean))
  (Variables|Default|SetAttackNumber AttackNumber)
  (Variables|Default|SetPlayerRef PlayerRef)
  (Variables|Default|SetDamageMultiplicator DamageMultiplicator)
  (Variables|Default|SetIs%20Heavy IsHeavy)
  (Utilities|Array|Clear (Variables|Default|GetIgnorList))
  (Variables|Default|SetIsAttacking true))

(event EventTick
  (params (DeltaSeconds :type Float%20%28single-precision%29))
  (bind _arrow (Variables|Default|GetArrow))
  (bind _playerstats (Variables|Default|GetPlayerStats))
  (bind (_lightattackdamage _jumplightmultiplier _backstabmultiplier _heavyattackbasedamage) (Utilities|Struct|BreakS_PlayerStats _playerstats))
  (bind _returnvalue (Transformation|GetWorldLocation _arrow))
  (if (Variables|Default|GetIsAttacking)
    (bind _outhit (Class|KismetSystemLibrary|CapsuleTraceSingleforObjects _returnvalue (+ _returnvalue (* (Math|Vector|GetForwardVector _arrow) 7e+01)) 2e+01 0.0 (Utilities|Array|MakeArray "ObjectTypeQuery7") false (Variables|Default|GetIgnorList) "ForDuration" true "(R=1.000000,G=0.000000,B=0.000000,A=1.000000)" "(R=0.000000,G=1.000000,B=0.000000,A=1.000000)" 0.2))
    (if (Utilities|DoesObjectImplementInterface (.HitActor (Collision|BreakHitResult _outhit)) "/Game/AI/BPI_Damageable.BPI_Damageable_C")
      (Utilities|Array|Add (Variables|Default|GetIgnorList) (.HitActor (Collision|BreakHitResult _outhit)))
      (Class|BPIDamageable|TAKEDamage(Message) (.HitActor (Collision|BreakHitResult _outhit)) (* (Variables|Default|GetDamageMultiplicator) (select (Variables|Default|GetIs%20Heavy) _heavyattackbasedamage _lightattackdamage)) (.ImpactPoint (Collision|BreakHitResult _outhit)) true "NewEnumerator0"))))

(fn ConstructionScript)