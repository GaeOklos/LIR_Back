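; Gameplay manager that initialises collectibles and enemy spawners, handles their respawn on bonfire reactivation, and runs a camera rewind time effect.
; Init caches the player, while Add events register collectibles and spawners into arrays.
; The first spawner registration triggers a delayed activation pass, staggered one spawner per tick.
; Rewind timelines ease global time dilation to near-freeze, reset AI and player stats, then restore normal speed.
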(event Custom|Add_Spawners
  (params (New_Spawner :type BP%20Enemy%20Spawner%20Object%20Reference))
  (Utilities|Array|Add (Variables|Default|GetEnemy_Spawners) New_Spawner)
  (Utilities|FlowControl|DoOnce false
    (:Completed
      (Utilities|FlowControl|Delay 2.0)
      (Variables|Default|Setcurrent_Index 0)
      (Variables|Default|SetSpawner_Index (Utilities|Array|Length (Variables|Default|GetEnemy_Spawners)))
      (CallFunction|SpawnEnemy))))

(event Custom|Reactivate_Bonefire
  (for _array_element (Variables|Default|GetResseources)
    (Default|RespawnRessource _array_element))
  (for _array_element_2 (Variables|Default|GetEnemy_Spawners)
    (Default|ActivateSpawners _array_element_2)))

(event Custom|Spawn_Enemy
  (bind _enemy_spawners (Variables|Default|GetEnemy_Spawners))
  (bind _current_index (Variables|Default|Getcurrent_Index))
  (bind _output (Utilities|Array|Get(acopy) _enemy_spawners _current_index))
  (Utilities|IsValid _output
    (:Is%20Valid
      (Default|ActivateSpawners _output)
      (Math|Integer|IncrementInt (Variables|Default|Getcurrent_Index)
        (:%20%20
          (Utilities|FlowControl|DelayUntilNextTick)
          (if (not (> (Variables|Default|Getcurrent_Index) (Variables|Default|GetSpawner_Index)))
            (CallFunction|SpawnEnemy)))))))

(event Custom|Start_Camera_Rewind
  (Components|Timeline|SetPlayRate (Variables|Default|GetTIMER_CameraRewind) (/ 1.0 1.75))
  (bind _alpha (Timeline|TIMER_CameraRewind PlayFromStart)
    (:Update
      (Utilities|Time|SetGlobalTimeDilation (Math|Float|Lerp 1.0 0.01 _alpha)))
    (:Finished
      (bind _outactors (Actor|GetAllActorsOfClass "/Game/AI/AIs/BP_AI_Master.BP_AI_Master_C"))
      (for _array_element _outactors
        (Default|CameraResetAllStatsAI _array_element))
      (Default|CameraFinalStats (Variables|Default|GetPLAYER))
      (Components|Timeline|SetPlayRate (Variables|Default|GetTIMER_EndRewind) (/ 1.0 1.5))
      (bind _alpha_2 (Timeline|TIMER_EndRewind PlayFromStart)
        (:Update
          (Utilities|Time|SetGlobalTimeDilation (Math|Float|Lerp 0.01 1.0 _alpha_2)))))))

(event Custom|AddCollectable
  (params (Collectible :type BP%20Collectable%20Master%20Object%20Reference))
  (Utilities|Array|Add (Variables|Default|GetResseources) Collectible))

(event Custom|Init
  (bind _asbp_player (Utilities|Casting|CastToBP_Player (Game|GetPlayerCharacter 0)))
  (Variables|Default|SetPLAYER _asbp_player)
  (CallFunction|InitialiseAll))

(event Custom|InitialiseAll
  (bind _outactors (Actor|GetAllActorsOfClass "/Game/Collectables/BP_CollectableMaster.BP_CollectableMaster_C"))
  (for _array_element _outactors
    (Default|Init _array_element))
  (bind _outactors_2 (Actor|GetAllActorsOfClass "/Game/AI/AIs/BP_Enemy_Spawner.BP_Enemy_Spawner_C"))
  (for _array_element_2 _outactors_2
    (Default|Init _array_element_2)))

(fn ConstructionScript)