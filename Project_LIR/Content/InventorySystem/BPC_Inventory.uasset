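; BPC_Inventory is an inventory component that stores item structs in an array and stacks items of the same name.
; AddToInventory calls Find, which rebuilds a list of item names on each call to locate the incoming item's index.
; A missing item is appended and an existing entry is overwritten, both passing through AddItemNum, whose graph holds a struct rebuild that sums the quantity.
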(event Custom|AddToInventory
  (params (Sitem :type S%20Item%20Structure) (Number :type Integer))
  (Variables|Default|SetSitemTemp Sitem)
  (Variables|Default|SetTempNumber Number)
  (bind _returnvalue (CallFunction|Find))
  (bind _output_get (Variables|Default|SetTempIndex _returnvalue))
  (if (< _output_get 0)
    (Utilities|Array|Add (Variables|Default|GetInventory) (Utilities|AddItemNum (Variables|Default|GetSitemTemp) (Variables|Default|GetTempNumber)))
    (else
      (Utilities|Array|SetArrayElem (Variables|Default|GetInventory) (Variables|Default|GetTempIndex) (Utilities|AddItemNum (Utilities|Array|Get(acopy) (Variables|Default|GetInventory) (Variables|Default|GetTempIndex)) (Variables|Default|GetTempNumber))))))

(fn Find
  (Utilities|Array|Clear (LocalVariables|GetItemTypeList))
  (for _array_element (Variables|Default|GetInventory)
    (Utilities|Array|Add (LocalVariables|GetItemTypeList) (Utilities|Struct|BreakS_Item _array_element)))
  (return (Utilities|Array|FindItem (LocalVariables|GetItemTypeList) (Utilities|Struct|BreakS_Item (Variables|Default|GetSitemTemp)))))