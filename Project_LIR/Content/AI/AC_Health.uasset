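; Actor component in the AI folder that tracks health and poise, with setup events for each maximum.
; Damage is subtracted from Health, and only the returned value is clamped, not the stored one.
; Poise works as a build-up meter: it starts at zero, accumulates damage up to MaxPoise and reports when full.
; Separate calls reset poise or overwrite either value directly, with no Tick logic.
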(event Custom|Setup_Health
  (params (NewHealth :type Float%20%28double-precision%29))
  (bind _output_get (Variables|Default|SetHealth NewHealth))
  (Variables|Default|SetMax_Health _output_get))

(event Custom|Setup_Poise
  (params (max_Poise :type Float%20%28double-precision%29))
  (Variables|Default|Setpoise 0.0)
  (Variables|Default|Setmax_Poise max_Poise))

(event Custom|Reset_Poise
  (Variables|Default|Setpoise 0.0))

(event EventBeginPlay)

(event EventTick
  (params (DeltaSeconds :type Float%20%28single-precision%29)))

(fn UpdateHealthDamage
  (params (Damage_Received :type Float%20%28double-precision%29))
  (bind _output_get (Variables|Default|SetHealth (- (Variables|Default|GetHealth) Damage_Received)))
  (return (Math|Float|Clamp(Float) _output_get 0.0 (Variables|Default|GetMax_Health))))

(fn UpdatePoiseHealth
  (params (Damage_Taken :type Float%20%28double-precision%29))
  (bind _max_poise (Variables|Default|Getmax_Poise))
  (bind _output_get (Variables|Default|Setpoise (Math|Float|Clamp(Float) (+ Damage_Taken (Variables|Default|Getpoise)) 0.0 _max_poise)))
  (return _output_get (== _output_get _max_poise)))

(fn UpdateValuePoise
  (params (New_poise :type Float%20%28double-precision%29))
  (Variables|Default|Setpoise New_poise))

(fn UpdateHealth
  (params (newHeath :type Float%20%28double-precision%29))
  (Variables|Default|SetHealth newHeath)
  (return (Variables|Default|GetHealth) (Variables|Default|GetMax_Health)))