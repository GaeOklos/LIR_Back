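; Enemy spawner actor that registers with GM_gameplay on Init and maintains a single spawned AI.
; Activation destroys any existing enemy, removing it from the player's AIList, then spawns the class found in DT_EnemyStats by enum-derived row name.
; The new enemy spawns above SpawnPoint with patrol points, stats row, sight settings and a spawner reference.
; It also stores a group manager owner, supports destroying its AI, and shows SpawnerName as a text label.
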(event Custom|Activate_Spawners
  (bind _spawnpoint (Variables|Default|GetSpawnPoint))
  (bind _actortospawn (Variables|Default|GetActorToSpawn))
  (bind _as_bp_player (Variables|Default|GetAs%20BP%20Player))
  (bind _returnvalue (Transformation|GetActorTransform _spawnpoint))
  (bind _returnvalue_2 (Utilities|String|EnumtoString _actortospawn))
  (bind _returnvalue_3 (Utilities|String|StringToName _returnvalue_2))
  (Utilities|IsValid (Variables|Default|GetSpawned_Actor)
    (:Is%20Valid
      (Utilities|IsValid _as_bp_player
        (:Is%20Valid
          (Utilities|Array|RemoveItem (Variables|/Game/Player/BP_Player.BP_Player_C|GetAIList _as_bp_player) (Variables|Default|GetSpawned_Actor))
          (Actor|DestroyActor (Variables|Default|GetSpawned_Actor)))
        (:Is%20Not%20Valid
          _)))
    (:Is%20Not%20Valid
      _))
  (bind _returnvalue_4 (Utilities|GetDataTableRow "/Game/AI/DT_EnemyStats.DT_EnemyStats" _returnvalue_3)
    (:then
      (bind _returnvalue_5 (Game|SpawnActorfromClass (.Enemy_Class (Utilities|Struct|BreakS_EnemyStats _returnvalue_4)) (Math|Transform|MakeTransform (+ (.location _returnvalue) "0.000000,0.000000,45.000000") (.rotation _returnvalue) "1.000000,1.000000,1.000000") "AdjustIfPossibleButAlwaysSpawn" "MultiplyWithRoot" 0 (Variables|Default|GetPatrolPoints) (Utilities|Struct|MakeDataTableRowHandle "/Game/AI/DT_EnemyStats.DT_EnemyStats" _returnvalue_3) (Variables|Default|GetAI_BaseSight) self (Variables|Default|Getdetect_Multi) 0))
      (Variables|Default|SetSpawned_Actor _returnvalue_5))))

(event Custom|Set_Group_Owner
  (params (Group_Owner :type BP%20Group%20Manager%20Object%20Reference))
  (Variables|Default|SetGroup_Manager_Owner Group_Owner))

(event Custom|Init
  (bind _asbp_player (Utilities|Casting|CastToBP_Player (Game|GetPlayerCharacter 0)))
  (Variables|Default|SetAs%20BP%20Player _asbp_player)
  (bind _asgm_gameplay (Utilities|Casting|CastToGM_gameplay (Game|GetGameMode)))
  (bind _output_get (Variables|Default|SetAs%20GM%20Gameplay _asgm_gameplay))
  (Default|AddSpawners _output_get self))

(event Custom|SPAWNER_Destroy_All_AI
  (Utilities|IsValid (Variables|Default|GetSpawned_Actor)
    (:Is%20Valid
      (Actor|DestroyActor (Variables|Default|GetSpawned_Actor))
      (Variables|Default|SetSpawned_Actor 0))))

(fn ConstructionScript
  (Rendering|Components|TextRender|SetText (Variables|Default|GetTextRender) (Variables|Default|GetSpawner_Name)))