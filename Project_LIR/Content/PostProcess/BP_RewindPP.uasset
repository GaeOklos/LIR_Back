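; BP_RewindPP handles the post-process transition for the rewind effect and registers itself with GM_gameplay on BeginPlay.
; Change_Rewind_PP plays or reverses a timeline that crossfades BlendWeight between the base and rewind volumes.
; IsRewiding is set but never cleared, and while true Tick writes empty settings to the base volume.
; Unconnected leftovers attempt per-setting lerps and material-based blending.
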(event Custom|Change_Rewind_PP
  (params (Rewind? :type Boolean))
  (if Rewind?
    (Variables|Default|SetisRewiding true))
  (Components|Timeline|SetPlayRate (Variables|Default|GetTIME_Change_Rewind_PP) (/ 1.0 0.4))
  (if Rewind?
    (bind _alpha (Timeline|TIME_Change_Rewind_PP PlayFromStart)
      (:Update
        (Variables|/Script/Engine.PostProcessVolume|SetBlendWeight (Variables|Default|GetPPBaseVolume) (Math|Float|Lerp 1.0 0.0 _alpha))
        (Variables|/Script/Engine.PostProcessVolume|SetBlendWeight (Variables|Default|GetPPRewindVolume) (Math|Float|Lerp 0.0 1.0 _alpha)))
      (:Finished
        (if (not Rewind?)
          (Variables|Default|SetisRewiding true))))
    (else
      (Timeline|TIME_Change_Rewind_PP Reverse))))

(event EventTick
  (params (DeltaSeconds :type Float%20%28single-precision%29))
  (if (Variables|Default|GetisRewiding)
    (Variables|/Script/Engine.PostProcessVolume|SetSettings (Variables|Default|GetPPBaseVolume) "")))

(event EventBeginPlay
  (Variables|Default|SetPPBase (Variables|/Script/Engine.PostProcessVolume|GetSettings (Variables|Default|GetPPBaseVolume)))
  (Variables|Default|SetPPRewind (Variables|/Script/Engine.PostProcessVolume|GetSettings (Variables|Default|GetPPRewindVolume)))
  (bind _asgm_gameplay (Utilities|Casting|CastToGM_gameplay (Game|GetGameMode)))
  (bind _output_get (Variables|Default|SetAs%20GM%20Gameplay _asgm_gameplay))
  (Variables|/Game/Player/GM_gameplay.GM_gameplay_C|Setpost_ProcressRewind _output_get self))

(fn ConstructionScript)