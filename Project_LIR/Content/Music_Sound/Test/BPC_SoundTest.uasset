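; BPC_SoundTest is a test Blueprint that toggles the W_Sound_Debug sound debug widget with the 7 key.
; An IsClose flag decides whether the event creates a fresh widget and adds it to the viewport or removes the stored one.
; Opening switches player 0 to game-and-UI input with a visible cursor, and closing restores game-only input and hides the cursor.
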(event Custom|Test_CreateWidget
  (bind _returnvalue (Game|GetPlayerController 0))
  (bind _returnvalue_2 (Game|GetPlayerController 0))
  (if (Variables|Default|Getis_Close)
    (Variables|Default|Setis_Close false)
    (bind _returnvalue_3 (UserInterface|CreateWidget "/Game/HUD/W_Sound_Debug.W_Sound_Debug_C" (Game|GetPlayerController 0)))
    (bind _output_get (Variables|Default|SetWidget_Ref _returnvalue_3))
    (UserInterface|Viewport|AddtoViewport _output_get 0)
    (Input|SetInputModeGameandUI _returnvalue_2 _output_get "DoNotLock" true false)
    (Variables|/Script/Engine.PlayerController|SetbShowMouseCursor _returnvalue_2 true)
    (else
      (Variables|Default|Setis_Close true)
      (Widget|RemovefromParent (Variables|Default|GetWidget_Ref))
      (Input|SetInputModeGameOnly _returnvalue false)
      (Variables|/Script/Engine.PlayerController|SetbShowMouseCursor _returnvalue false))))

(event Input|KeyboardEvents|7
  (params (Key :type Key%20Structure :default "None"))
  (:Pressed
    (CallFunction|TestCreateWidget)))