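; Test actor component that spirals its owner up and outward around a target actor, then releases it to physics.
; StartMovement records the target and horizontal radius, then Tick advances the angle and multiplicatively grows climb and radius rates, with climb capped.
; RotateActorAroundPoint repositions and rotates the owner each frame, with optional debug lines.
; At a max radius randomized on BeginPlay, orbiting stops and BP_Transportable_Test's mesh simulates physics; the impulse is unwired.
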(event Custom|StartMovement
  (params (ActorToRotateTo :type Actor%20Object%20Reference))
  (bind _owner (Variables|Default|GetOwner))
  (bind _returnvalue (Transformation|GetActorLocation _owner))
  (Variables|Default|SetTargetAction ActorToRotateTo)
  (Variables|Default|SetInitialLocation (Math|Vector|MakeVector (.x _returnvalue) (.y _returnvalue) (.z _returnvalue)))
  (Variables|Default|SetRadius (Math|Vector|VectorLength (- (Math|Vector|MakeVector (.x (Transformation|GetActorLocation (Variables|Default|GetTargetAction))) (.y (Transformation|GetActorLocation (Variables|Default|GetTargetAction))) (.z _returnvalue)) (Math|Vector|MakeVector (.x _returnvalue) (.y _returnvalue) (.z _returnvalue)))))
  (Variables|Default|Setis_Rotating true))

(event Custom|Propulstion
  (params (Will :type Vector))
  (Variables|Default|Setis_Rotating false)
  (bind _asbp_transportable_test (Utilities|Casting|CastToBP_Transportable_Test (Variables|Default|GetOwner)))
  (Physics|SetSimulatePhysics (Variables|/Game/Music_Sound/Test/BP_Transportable_Test.BP_Transportable_Test_C|GetStaticMesh _asbp_transportable_test) true))

(event EventBeginPlay
  (Variables|Default|SetOwner (Components|GetOwner))
  (bind _output_get (Variables|Default|SetMaxRadius (Math|Random|RandomFloatinRange (/ (Variables|Default|GetMaxRadius) 1e+02) (Variables|Default|GetMaxRadius))))
  (Development|PrintString (Utilities|String|ToString(Float) _output_get)))

(event EventTick
  (params (DeltaSeconds :type Float%20%28single-precision%29))
  (if (Variables|Default|Getis_Rotating)
    ;[1 1 1] Set Up for Rotating
    ;;[1 1 1] RotationSpeed
    (Variables|Default|SetCurrentRotation_Rate (+ (Variables|Default|GetCurrentRotation_Rate) (* (* (Variables|Default|GetRotationSpeed) DeltaSeconds) (Math|Float|SelectFloat 1.0 -1.0 (Variables|Default|GetClockwise)))))
    ;;[1 1 1] Height
    (if (<= (Variables|Default|GetMaxSpeed_Height) (Variables|Default|GetEvolutionCurrentHeightRate))
      _
      (else
        (bind _output_get (Variables|Default|SetEvolutionCurrentHeightRate (* (Variables|Default|GetEvolutionSpeed_Height) (Variables|Default|GetEvolutionCurrentHeightRate))))))
    ;;[1 0.6811 0.5806] Radius
    (if (<= (Variables|Default|GetMaxRadius) (+ (Variables|Default|GetRadius) (Variables|Default|GetEvolutionCurrentRateRadius)))
      (Variables|Default|SetIs_Propulsion true)
      (else
        (Variables|Default|SetEvolutionCurrentRateRadius (* (Variables|Default|GetEvolutionSpeed_Radius) (Variables|Default|GetEvolutionCurrentRateRadius)))))
    ;[0.02985 1 0.9502] Rotating
    (bind (_location _destinationpoint) (CallFunction|RotateActorAroundPoint (Variables|Default|GetInitialLocation)))
    (if (Variables|Default|GetIs_Propulsion)
      (CallFunction|Propulstion _destinationpoint)
      (elif (Variables|Default|GetDrawDebug)
        (Rendering|Debug|DrawDebugLine _location (Transformation|GetActorLocation (Variables|Default|GetOwner)) (Variables|Default|GetLine%20Color) 1.0 2.0)))))

(fn RotateActorAroundPoint
  (params (L_Location :type Vector))
  (bind _targetaction (Variables|Default|GetTargetAction))
  (bind _owner (Variables|Default|GetOwner))
  (bind _returnvalue (Transformation|GetActorLocation _targetaction))
  (LocalVariables|SetTmp_Location_Target L_Location)
  (LocalVariables|SetTmp_Location_Target (Math|Vector|MakeVector (.x _returnvalue) (.y _returnvalue) (+ (.z (Transformation|GetActorLocation (Variables|Default|GetOwner))) (Variables|Default|GetEvolutionCurrentHeightRate))))
  (bind _output_get (LocalVariables|SetDestination (+ (LocalVariables|GetTmp_Location_Target) (Math|Vector|RotateVectorAroundAxis (Math|Vector|MakeVector (+ (Variables|Default|GetRadius) (Variables|Default|GetEvolutionCurrentRateRadius)) 0.0 0.0) (+ (Variables|Default|GetCurrentRotation_Rate) (Variables|Default|GetStartingAngle)) "0.000000,0.000000,1.000000"))))
  (Transformation|SetActorLocation _owner _output_get false false)
  (Class|Actor|AddActorWorldRotation _owner (Math|Rotator|MakeRotator 0.0 (+ (.yaw (Transformation|GetActorRotation _owner)) 0.5) 0.0))
  (return (LocalVariables|GetTmp_Location_Target) (LocalVariables|GetDestination)))