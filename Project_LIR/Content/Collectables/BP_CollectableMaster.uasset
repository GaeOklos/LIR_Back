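; Base collectable actor that the player interacts with to add an item to their inventory.
; The construction script fills the item data from a DT_Item row and sets its mesh, or an override mesh and material.
; Interaction hides the mesh, marks ACInteractif used, adds the item to the instigator's inventory and shows it in the UI.
; Init registers it with GM_gameplay, and RespawnRessource makes a used collectable visible and usable again.
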(event Custom|RespawnRessource
  (if (Variables|/Game/Interactif/AC_Interactif.AC_Interactif_C|GetisUsed? (Variables|Default|GetAC_Interactif))
    (Rendering|SetVisibility (Variables|Default|GetStaticMesh) true true)
    (Default|ChangeUsageState (Variables|Default|GetAC_Interactif) false)))

(event Custom|Init
  (bind _asgm_gameplay (Utilities|Casting|CastToGM_gameplay (Game|GetGameMode)))
  (bind _output_get (Variables|Default|SetAs%20GM%20Gameplay _asgm_gameplay))
  (Default|AddCollectable _output_get self))

(event EventStartInteraction
  (params (Instigator :type BP%20Player%20Object%20Reference))
  (bind _numbertoadd (Variables|Default|GetNumberToAdd))
  (bind _itemtype (Variables|Default|GetItemType))
  (bind (_item _itemname _icon) (Utilities|Struct|BreakS_Item _itemtype))
  (if (not (Variables|/Game/Interactif/AC_Interactif.AC_Interactif_C|GetisUsed? (Variables|Default|GetAC_Interactif)))
    (Rendering|SetVisibility (Variables|Default|GetStaticMesh) false true)
    (Default|ChangeUsageState (Variables|Default|GetAC_Interactif) true)
    (Default|AddtoInventory (Variables|/Game/Player/BP_Player.BP_Player_C|GetBPC_Inventory Instigator) (Variables|Default|GetItemType) _numbertoadd)
    (Default|GetItemCE (Variables|/Game/Player/BP_Player.BP_Player_C|GetMainWidgetUIN Instigator) (Utilities|Text|ToText(Name) _itemname) (Utilities|String|ToString(Integer) _numbertoadd) _icon)))

(fn ConstructionScript
  (bind _staticmesh (Variables|Default|GetStaticMesh))
  (bind _returnvalue (Utilities|GetDataTableRow "/Game/InventorySystem/DT_Item.DT_Item" (.rowname (Variables|Default|GetDataRow)))
    (:then
      (Variables|Default|SetItemType (Utilities|Struct|MakeS_Item (.item _returnvalue) (.itemname _returnvalue) (.icon _returnvalue) (.mesh _returnvalue) (.number _returnvalue) (.itemtype _returnvalue) (.itemeffect _returnvalue) (.obtained _returnvalue)))
      (if (Variables|Default|GetOverrideModel)
        (Components|StaticMesh|SetStaticMesh _staticmesh (Variables|Default|GetMesh))
        (Rendering|Material|SetMaterial (Variables|Default|GetStaticMesh) 0 (Variables|Default|GetMaterial))
        (else
          (Components|StaticMesh|SetStaticMesh _staticmesh (.mesh _returnvalue)))))))